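; Character Blueprint for AVoid that handles the wind and splash audio tied to death and restart.
; On BeginPlay it binds handlers to the character dead and restart delegates, then stops both audio components.
; The death audio function fades out the wind and plays the splash, while the restart function calls a fade-in and then Play on the wind.
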(event EventBeginPlay
  (EventDispatchers|BindEventtoOnCharacterDeadDelegate (EventDispatchers|CreateEvent :!event OnDeathAudio))
  (EventDispatchers|BindEventtoOnCharacterRestartDelegate (EventDispatchers|CreateEvent :!event OnRestartAudio))
  (Audio|Components|Audio|Stop (Variables|Default|GetSplashAudio)))

(fn ConstructionScript)

(fn OnDeathAudio
  (Audio|Components|Audio|FadeOut (Variables|Default|GetWindAudio) 1.0 0.0 "Linear" :!class /Script/Engine.AudioComponent)
  (Audio|Components|Audio|Play (Variables|Default|GetSplashAudio) 0.0))

(fn OnRestartAudio
  (bind _windaudio (Variables|Default|GetWindAudio))
  (Audio|Components|Audio|FadeIn _windaudio 2.0 1.0 0.0 "Linear" :!class /Script/Engine.AudioComponent)
  (Audio|Components|Audio|Play _windaudio 0.0))