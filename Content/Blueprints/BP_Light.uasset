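; BP_Light is a point light actor that reacts when something other than a VoidCharacter overlaps its static mesh.
; It applies its configured intensity on BeginPlay.
; On a failed VoidCharacter cast, it sets a target slightly offset from the Character's location and briefly flashes the light brighter and red.
; After a short delay, it restores the base intensity and white color.
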(event OnComponentBeginOverlap(StaticMesh)
  (params (OverlappedComponent :type Primitive%20Component%20Object%20Reference) (OtherActor :type Actor%20Object%20Reference) (OtherComp :type Primitive%20Component%20Object%20Reference) (OtherBodyIndex :type Integer) (bFromSweep :type Boolean) (SweepResult :type Hit%20Result%20Structure%20%28by%20ref%29))
  (bind _pointlight (Variables|Default|GetPointLight))
  (bind _pointlight_2 (Variables|Default|GetPointLight))
  (Utilities|Casting|CastToAVoidCharacter OtherActor
    (:CastFailed
      (Class|CharacterLight|SetTarget (+ (Transformation|GetActorLocation (Variables|Default|GetCharacter)) "15.000000, 0, 0"))
      (Rendering|Components|Light|SetIntensity _pointlight (* 5 (Variables|Default|GetIntensity)))
      (Rendering|Components|Light|SetLightColor _pointlight "(R=1.000000,G=0.000000,B=0.000000,A=1.000000)" true)
      (Utilities|FlowControl|Delay 0.2)
      (Rendering|Components|Light|SetIntensity _pointlight_2 (Variables|Default|GetIntensity))
      (Rendering|Components|Light|SetLightColor _pointlight_2 "(R=1.000000,G=1.000000,B=1.000000,A=1.000000)" true))))

(event EventBeginPlay
  (Rendering|Components|Light|SetIntensity (Variables|Default|GetPointLight) (Variables|Default|GetIntensity)))

(event Collision|EventActorBeginOverlap
  (params (OtherActor :type Actor%20Object%20Reference)))

(event EventTick
  (params (DeltaSeconds :type Float%20%28single-precision%29)))

(fn ConstructionScript)